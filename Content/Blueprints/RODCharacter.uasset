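; Character Blueprint that handles the melee hits RODCharacter deals to Enemigo enemies.
; The construction script attaches a hand collision component to the mesh's RightHand socket.
; When it overlaps an enemy's capsule during a melee attack, the enemy's life is updated with the melee damage.
; Each hit also turns CanBeDamaged off, then restores it after a short delay.
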(event `self.RightHandCollision.OnComponentBeginOverlap`
  (params (OverlappedComponent :type "PrimitiveComponent Object Reference") (OtherActor :type "Actor Object Reference") (OtherComp :type "PrimitiveComponent Object Reference") (OtherBodyIndex :type Integer) (bFromSweep :type Boolean) (SweepResult :type "HitResult Structure (by ref)"))
  ;[1 1 1] Update enemy life when is Melee hitted
  (bind _asenemigo (cast `Enemigo` OtherActor))
  (if (== (`Character.CapsuleComponent` _asenemigo) OtherComp)
    (set `self.bCanBeDamaged` (`self.CanBeDamaged`))
    (if (`self.IsInMeleeAttack`)
      (set `self.CanBeDamaged` false)
      (`Enemigo.UpdateLife` _asenemigo (`self.GetMeleeDamage`))
      (`KismetSystemLibrary.Delay` 0.98)
      (set `self.CanBeDamaged` true))))

(fn `UserConstructionScript`
  ;[1 1 1] Atacched Mesh Colision
  (`SceneComponent.K2_AttachToComponent` (`self.RightHandCollision`) (`self.Mesh`) "RightHand" "KeepRelative" "KeepRelative" "KeepRelative" true))