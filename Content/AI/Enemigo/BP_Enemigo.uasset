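; Enemy character Blueprint with an overhead health bar and a hit reaction.
; Each tick it writes Health as a fraction of 100 to the widget's progress bar and yaws the widget toward the player camera.
; On a Hit event, if the hit actor is an Enemigo, it pulses that actor's AnimBP Hitted flag for half a second.
; The construction script attaches RightHandCollision to the mesh's RightHand socket.
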(event `self.ReceiveTick`
  (params (DeltaSeconds :type "Float (single-precision)"))
  ;[1 1 1] Barra salud enemigo
  (bind _aswidget_estado_enemigo (cast `/Game/AI/Enemigo/WidgetEstadoEnemigo` (`WidgetComponent.GetUserWidgetObject` (`self.WidgetSalud`))))
  (`ProgressBar.SetPercent` (`/Game/AI/Enemigo/WidgetEstadoEnemigo.ProgressBar_165` _aswidget_estado_enemigo) (/ (`self.Health`) 100.0))
  (`SceneComponent.K2_SetWorldRotation` (`self.Widgetsalud`) (`KismetMathLibrary.MakeRotator` 0.0 0.0 (.yaw (`KismetMathLibrary.FindLookAtRotation` (`SceneComponent.K2_GetComponentLocation` (`self.Widgetsalud`)) (`self.K2_GetActorLocation` (`GameplayStatics.GetPlayerCameraManager` (`GameplayStatics.GetPlayerCharacter` 0)))))) false false))

(event `self.ReceiveHit`
  (params (MyComp :type "PrimitiveComponent Object Reference") (Other :type "Actor Object Reference") (OtherComp :type "PrimitiveComponent Object Reference") (bSelfMoved :type Boolean) (HitLocation :type "Vector Structure") (HitNormal :type "Vector Structure") (NormalImpulse :type "Vector Structure") (Hit :type "HitResult Structure (by ref)"))
  (bind _asenemigo (cast `Enemigo` (`.HitActor` (`GameplayStatics.BreakHitResult` Hit))))
  (bind _asthird_person_anim_bp (cast `/Game/Mannequin/Animations/ThirdPerson_AnimBP` (`SkeletalMeshComponent.GetAnimInstance` (`Character.Mesh` _asenemigo))))
  (set `/Game/Mannequin/Animations/ThirdPerson_AnimBP.Hitted?` true _asthird_person_anim_bp)
  (`KismetSystemLibrary.Delay` 0.5)
  (set `/Game/Mannequin/Animations/ThirdPerson_AnimBP.Hitted?` false _asthird_person_anim_bp))

(fn `UserConstructionScript`
  (`SceneComponent.K2_AttachToComponent` (`self.RightHandCollision`) (`self.Mesh`) "RightHand" "KeepRelative" "KeepRelative" "KeepRelative" true))