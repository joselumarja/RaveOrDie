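; Melee enemy (ZombieBoy) that damages the RODCharacter with its right hand and shows a health bar.
; The construction script attaches RightHandCollision to the mesh's RightHand socket.
; After a short delay, an overlap with the player's capsule calls UpdateLife with GetMeleeDamage, using the enemy's own CanBeDamaged flag as a hit cooldown.
; Tick refreshes the widget's progress bar from Health and holds it at a fixed world rotation.
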(event `self.ReceiveTick`
  (params (DeltaSeconds :type "Float (single-precision)"))
  ;[1 1 1] Actualizar Barra de vida
  (bind _aswidget_estado_enemigo (cast `/Game/AI/Enemigo/WidgetEstadoEnemigo` (`WidgetComponent.GetUserWidgetObject` (`self.BarraSalud`))))
  (`ProgressBar.SetPercent` (`/Game/AI/Enemigo/WidgetEstadoEnemigo.ProgressBar_165` _aswidget_estado_enemigo) (/ (`self.Health`) 100.0))
  (`SceneComponent.K2_SetWorldRotation` (`self.BarraSalud`) (struct :`Pitch` 45.0 :`Yaw` 180.0) false false))

(event `self.RightHandCollision.OnComponentBeginOverlap`
  (params (OverlappedComponent :type "PrimitiveComponent Object Reference") (OtherActor :type "Actor Object Reference") (OtherComp :type "PrimitiveComponent Object Reference") (OtherBodyIndex :type Integer) (bFromSweep :type Boolean) (SweepResult :type "HitResult Structure (by ref)"))
  (`KismetSystemLibrary.Delay` 0.2)
  (bind _asrodcharacter (cast `RODCharacter` OtherActor))
  (if (== (`Character.CapsuleComponent` _asrodcharacter) OtherComp)
    (if (`self.bCanBeDamaged`)
      (set `self.bCanBeDamaged` false)
      (`RODCharacter.UpdateLife` _asrodcharacter (`self.GetMeleeDamage`))
      (`KismetSystemLibrary.Delay` 0.83)
      (set `self.bCanBeDamaged` true))))

(fn `UserConstructionScript`
  (`SceneComponent.K2_AttachToComponent` (`self.RightHandCollision`) (`self.Mesh`) "RightHand" "KeepRelative" "KeepRelative" "KeepRelative" true))